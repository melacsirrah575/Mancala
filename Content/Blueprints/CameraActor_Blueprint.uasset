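; Camera actor that switches its view orientation according to whose turn it is.
; It caches the MainGameMode on BeginPlay, then checks its PlayersTurn flag every Tick.
; Each branch waits on a one-second Delay before snapping the CameraComponent to one of two fixed world rotations, with no interpolation.
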(event `self.ReceiveBeginPlay`
  (bind _asmain_game_mode (cast `/Game/Blueprints/MainGameMode` (`GameplayStatics.GetGameMode`)))
  (set `self.MainGameMode` _asmain_game_mode))

(event `self.ReceiveTick`
  (params (DeltaSeconds :type "Float (single-precision)"))
  (bind _cameracomponent (`self.CameraComponent`))
  (if (`/Game/Blueprints/MainGameMode.PlayersTurn` (`self.MainGameMode`))
    (`KismetSystemLibrary.Delay` 1.0)
    (`SceneComponent.K2_SetWorldRotation` _cameracomponent (struct :`Pitch` -90.0 :`Roll` -270.0) false false)
    (else
      (`KismetSystemLibrary.Delay` 1.0)
      (`SceneComponent.K2_SetWorldRotation` _cameracomponent (struct :`Pitch` -90.0 :`Roll` 270.0) false false))))

(fn `UserConstructionScript`)