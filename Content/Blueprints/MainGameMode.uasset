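; Game mode for a Mancala game that sows the stones from a selected pit by spawning stone actors around the board.
; SpawnStonesFromSelectedPit loops over StonesToSpawn, stepping and wrapping StoneSpawnIndex through the spawner array.
; At each side's end pit, CheckSpawnStoneInMancala can drop a stone into the current side's Mancala, nudging it with an impulse against stacking.
; A last stone landing there adjusts PlayersTurn, intended as an extra turn.
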(event `GetStoneSpawnLocationAndSpawnStone`
  ;[1 1 1] Get StoneSpawnIndex for ForLoop and Spawn Stone
  (if (and (>= (`self.StoneSpawnIndex`) 6) (== (`self.PlayersTurn`) true))
    (`|SpawnActorFromClass` "/Game/Blueprints/Stone.Stone_C" (`KismetMathLibrary.Conv_VectorToTransform` (`self.K2_GetActorLocation` (`|GetArrayItem` (`self.StoneSpawnerArray`) (`self.StoneSpawnIndex`)))) "Undefined" "OverrideRootScale" null null)
    (elif (and (<= (`self.StoneSpawnIndex`) 5) (== (`self.PlayersTurn`) false))
      (`|SpawnActorFromClass` "/Game/Blueprints/Stone.Stone_C" (`KismetMathLibrary.Conv_VectorToTransform` (`self.K2_GetActorLocation` (`|GetArrayItem` (`self.StoneSpawnerArray`) (`self.StoneSpawnIndex`)))) "Undefined" "OverrideRootScale" null null)
      (elif (and (<= (`self.StoneSpawnIndex`) 5) (== (`self.HasIncremented`) true))
        (`|SpawnActorFromClass` "/Game/Blueprints/Stone.Stone_C" (`KismetMathLibrary.Conv_VectorToTransform` (`self.K2_GetActorLocation` (`|GetArrayItem` (`self.StoneSpawnerArray`) (`self.StoneSpawnIndex`)))) "Undefined" "OverrideRootScale" null null)
        (if (== (`self.ForLoopIndex`) (`self.StonesToSpawn`))
          (set `self.HasIncremented` false))
        (else
          (`|SpawnActorFromClass` "/Game/Blueprints/Stone.Stone_C" (`KismetMathLibrary.Conv_VectorToTransform` (`self.K2_GetActorLocation` (`|GetArrayItem` (`self.StoneSpawnerArray`) (+ (`self.StoneSpawnIndex`) 1)))) "Undefined" "OverrideRootScale" null null))))))

(event `SpawnStonesFromSelectedPit`
  (for _index (range 1 (+ (`self.StonesToSpawn`) 1))
    (set `self.ForLoopIndex` _index)
    ;[1 1 1] Spawn Stones From Selected Pit
    (if (and (== (`self.StoneSpawnIndex`) 11) (== (`self.PlayersTurn`) true))
      (set `self.HasIncremented` true)
      (`self.GetStoneSpawnLocationAndSpawnStone` :!label _label)
      (`/Engine/EditorBlueprintResources/StandardMacros.IncrementInt` (`self.StoneSpawnIndex`))
      (else
        (if (== (`self.StoneSpawnIndex`) 11)
          _
          (elif (not (< (`self.StoneSpawnIndex`) 11))
            (set `self.StoneSpawnIndex` 0)))
        (if (or (and (== (`self.StonesToSpawn`) 1) (or (== (`self.StoneSpawnIndex`) 5) (== (`self.StoneSpawnIndex`) 11))) (or (== (`self.StoneSpawnIndex`) 5) (== (`self.StoneSpawnIndex`) 11)))
          (`self.CheckSpawnStoneInMancala`)
          (else
            (goto _label))))))
  (set `self.StonesToSpawn` 0))

(event `CheckSpawnStoneInMancala`
  (bind _output (`|GetArrayItem` (`self.MancalaArray`) (`self.MancalaIndex`)))
  ;[1 0.9646 0.604] SpawnStoneInMancala
  ;;[1 0.3561 0.456] Checks if Mancala is next spawnpoint based on whose turn it is
  (if (`self.PlayersTurn`)
    (if (and (<= (`self.ForLoopIndex`) (`self.StonesToSpawn`)) (== (`self.StoneSpawnIndex`) 5))
      (set `self.MancalaIndex` 1)
      ;;[1 1 1] Spawns Stone and prevents stacking
      (bind _returnvalue (`|SpawnActorFromClass` "/Game/Blueprints/Stone.Stone_C" (`KismetMathLibrary.Conv_VectorToTransform` (`self.K2_GetActorLocation` _output)) "Undefined" "OverrideRootScale" _output null :!label _label_2))
      (`PrimitiveComponent.AddImpulse` (`/Game/Blueprints/Stone.StoneBody` _returnvalue) (0.0 10.0 0.0) "None" false)
      ;;[1 1 1] Reduces ForLoop by 1 and gives player a second turn if their last stone ended in their Mancala
      (if (and (== (`self.ForLoopIndex`) (`self.StonesToSpawn`)) (== (`self.StoneSpawnIndex`) 5) (== (`self.PlayersTurn`) true))
        (set `self.PlayersTurn` false)
        (elif (and (== (`self.ForLoopIndex`) (`self.StonesToSpawn`)) (== (`self.StoneSpawnIndex`) 11) (== (`self.PlayersTurn`) false))
          (set `self.PlayersTurn` true)
          (else
            (`/Engine/EditorBlueprintResources/StandardMacros.IncrementInt` (`self.StoneSpawnIndex`)
              (:`  `
                (if (== (`self.StonesToSpawn`) 0)
                  (if (`self.PlayersTurn`)
                    (set `self.PlayersTurn` false)
                    (else
                      (set `self.PlayersTurn` true))))))))))
    (elif (and (<= (`self.ForLoopIndex`) (`self.StonesToSpawn`)) (== (`self.StoneSpawnIndex`) 11))
      (set `self.MancalaIndex` 0)
      (goto _label_2))))

(fn `UserConstructionScript`)