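; Pits is a board pit actor that holds Stone actors and responds to the mouse.
; Cursor hover toggles visibility of its particle system and the touched component.
; Clicking the sphere counts overlapping stones and reveals that number in the StoneCount text.
; An unconnected loop, noted as not working, would hide stones, disable gravity and teleport them to the MainGameMode's presentation location.
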(event `self.ReceiveBeginPlay`
  ;[1 1 1] Cast To MainGameMode
  (bind _asmain_game_mode (cast `/Game/Blueprints/MainGameMode` (`GameplayStatics.GetGameMode`)))
  (set `self.MainGameMode` _asmain_game_mode))

(event `self.Sphere.OnBeginCursorOver`
  (params (TouchedComponent :type "PrimitiveComponent Object Reference"))
  ;[1 1 1] Handles Particle System On Cursor Over
  (`SceneComponent.SetVisibility` (`self.ParticleSystem`) true true)
  (`SceneComponent.SetVisibility` TouchedComponent true true))

(event `self.Sphere.OnEndCursorOver`
  (params (TouchedComponent :type "PrimitiveComponent Object Reference"))
  ;[1 1 1] Handles Particle System On Cursor Over
  (`SceneComponent.SetVisibility` (`self.ParticleSystem`) false false)
  (`SceneComponent.SetVisibility` TouchedComponent false false))

(event `self.Sphere.OnClicked`
  (params (TouchedComponent :type "PrimitiveComponent Object Reference") (ButtonPressed :type "Key Structure"))
  (bind _stonecount (`self.StoneCount`))
  (`TextRenderComponent.K2_SetText` _stonecount (`KismetTextLibrary.Conv_IntToText` (+ (`KismetArrayLibrary.Array_LastIndex` (`PrimitiveComponent.GetOverlappingActors` (`self.Sphere`) "/Game/Blueprints/Stone.Stone_C")) 1)))
  (`SceneComponent.SetHiddenInGame` _stonecount false false))

(fn `UserConstructionScript`)