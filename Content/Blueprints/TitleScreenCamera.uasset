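; Title screen camera actor that glides toward an end point while keeping the Mancala board in view.
; BeginPlay caches the game mode, start location and EndPoint's world location.
; Each Tick re-aims the scene component at the MancalaBoard via look-at rotation and moves the actor toward the cached point with constant-speed interpolation.
; Unconnected logic for showing the TitleScreen widget on arrival never runs.
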(event `self.ReceiveBeginPlay`
  (bind _asmain_game_mode (cast `/Game/Blueprints/MainGameMode` (`GameplayStatics.GetGameMode`)))
  (set `self.MainGameMode` _asmain_game_mode)
  (set `self.CurrentLocation` (`self.K2_GetActorLocation`))
  (set `self.EndPointLocation` (`SceneComponent.K2_GetComponentLocation` (`self.EndPoint`))))

(event `self.ReceiveTick`
  (params (DeltaSeconds :type "Float (single-precision)"))
  (bind _scenecomponent (`self.SceneComponent`))
  (bind _returnvalue (`GameplayStatics.GetActorOfClass` "/Game/Blueprints/MancalaBoard.MancalaBoard_C"))
  (`SceneComponent.K2_SetWorldRotation` _scenecomponent (`KismetMathLibrary.FindLookAtRotation` (`SceneComponent.K2_GetComponentLocation` _scenecomponent) (`self.K2_GetActorLocation` _returnvalue)) false false)
  (set `self.DeltaTime` DeltaSeconds)
  (bind _output_get (set `self.CurrentLocation` (`KismetMathLibrary.VInterpTo_Constant` (`self.CurrentLocation`) (`self.EndPointLocation`) (`self.DeltaTime`) (`self.MovementSpeed`))))
  (`self.K2_SetActorLocation` _output_get))

(fn `UserConstructionScript`)