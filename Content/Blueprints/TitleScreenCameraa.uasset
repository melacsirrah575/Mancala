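; Title screen camera actor that flies to a preset end point while facing the Mancala board, then shows the title screen.
; BeginPlay caches the game mode and the EndPoint component's world location as a fixed target.
; Each tick it moves the actor at constant speed and re-aims the camera at the board, looked up by class every frame.
; On reaching the target, a DoOnce creates the TitleScreen widget and adds it to the viewport.
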(event `self.ReceiveBeginPlay`
  (bind _asmain_game_mode (cast `/Game/Blueprints/MainGameMode` (`GameplayStatics.GetGameMode`)))
  (set `self.MainGameMode` _asmain_game_mode)
  (set `self.CurrentLocation` (`self.K2_GetActorLocation`))
  (set `self.EndPointLocation` (`SceneComponent.K2_GetComponentLocation` (`self.End Point`))))

(event `self.ReceiveTick`
  (params (DeltaSeconds :type "Float (single-precision)"))
  (bind _camera (`self.Camera`))
  (set `self.DeltaTime` DeltaSeconds)
  (bind _output_get (set `self.CurrentLocation` (`KismetMathLibrary.VInterpTo_Constant` (`self.CurrentLocation`) (`self.EndPointLocation`) (`self.DeltaTime`) (`self.MovementSpeed`))))
  (`self.K2_SetActorLocation` _output_get)
  (bind _returnvalue (`GameplayStatics.GetActorOfClass` "/Game/Blueprints/MancalaBoard.MancalaBoard_C"))
  (`SceneComponent.K2_SetWorldRotation` _camera (`KismetMathLibrary.FindLookAtRotation` (`SceneComponent.K2_GetComponentLocation` _camera) (`self.K2_GetActorLocation` _returnvalue)) false false)
  (if (<= (`KismetMathLibrary.VSize` (- (`self.K2_GetActorLocation`) (`self.EndPointLocation`))) 0.0)
    (`/Engine/EditorBlueprintResources/StandardMacros.DoOnce` false
      (:`Completed`
        (bind _returnvalue_2 (`|CreateWidget` "/Game/UI/TitleScreen.TitleScreen_C"))
        (`UserWidget.AddToViewport` _returnvalue_2 0)))))

(fn `UserConstructionScript`)