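; Mancala board actor that shows how many stones lie inside its counter volume when the cursor hovers over it.
; On hover it flips the whole actor's roll to match the current turn from MainGameMode, then reveals a text render with the count.
; The count comes from Stone actors overlapping StoneCounter, recomputed on each hover begin and end, with the text hidden again when the cursor leaves.
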(event `self.ReceiveBeginPlay`
  (bind _asmain_game_mode (cast `/Game/Blueprints/MainGameMode` (`GameplayStatics.GetGameMode`)))
  (set `self.MainGameMode` _asmain_game_mode))

(event `self.StoneCounter.OnBeginCursorOver`
  (params (TouchedComponent :type "PrimitiveComponent Object Reference"))
  (bind _textrender (`self.TextRender`))
  (if (`/Game/Blueprints/MainGameMode.PlayersTurn` (`self.MainGameMode`))
    (`self.K2_SetActorRotation` (struct))
    (else
      (`self.K2_SetActorRotation` (struct :`Yaw` 180.0))))
  ;[1 1 1] Sets Text and Visibility on Hover
  (`TextRenderComponent.K2_SetText` _textrender (`KismetTextLibrary.Conv_IntToText` (+ (`KismetArrayLibrary.Array_LastIndex` (`PrimitiveComponent.GetOverlappingActors` (`self.StoneCounter`) "/Game/Blueprints/Stone.Stone_C")) 1)))
  (`SceneComponent.SetHiddenInGame` _textrender false false))

(event `self.StoneCounter.OnEndCursorOver`
  (params (TouchedComponent :type "PrimitiveComponent Object Reference"))
  (bind _textrender (`self.TextRender`))
  ;[1 1 1] Sets Text and Visibility on Hover
  (`TextRenderComponent.K2_SetText` _textrender (`KismetTextLibrary.Conv_IntToText` (+ (`KismetArrayLibrary.Array_LastIndex` (`PrimitiveComponent.GetOverlappingActors` (`self.StoneCounter`) "/Game/Blueprints/Stone.Stone_C")) 1)))
  (`SceneComponent.SetHiddenInGame` _textrender true false))

(fn `UserConstructionScript`)